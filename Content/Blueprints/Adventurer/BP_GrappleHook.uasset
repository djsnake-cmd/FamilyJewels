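; BP_GrappleHook is the adventurer's grapple hook projectile, with its launch speed set from ProjectileSpeed in the construction script.
; On hit, it writes the player adventurer's location and the hit location as grapple start and end points, then calls MoveGrapple on that character.
; It then polls the character's movement mode on a short repeating delay and destroys itself once the mode is not None.
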(event `self.ReceiveHit`
  (params (MyComp :type "PrimitiveComponent Object Reference") (Other :type "Actor Object Reference") (OtherComp :type "PrimitiveComponent Object Reference") (bSelfMoved :type Boolean) (HitLocation :type "Vector Structure") (HitNormal :type "Vector Structure") (NormalImpulse :type "Vector Structure") (Hit :type "HitResult Structure (by ref)"))
  (bind _asbp_adventurer (cast `/Game/Blueprints/Adventurer/BP_Adventurer` (`GameplayStatics.GetPlayerCharacter` 0)))
  (set `/Game/Blueprints/Adventurer/BP_Adventurer.GrappleStartLoc` (`self.K2_GetActorLocation` _asbp_adventurer) _asbp_adventurer)
  (set `/Game/Blueprints/Adventurer/BP_Adventurer.GrappleEndLoc` HitLocation _asbp_adventurer)
  (`/Game/Blueprints/Adventurer/BP_Adventurer.MoveGrapple` _asbp_adventurer)
  (`KismetSystemLibrary.Delay` 0.1 :!label _label)
  (if (`|EnumInequality` (`CharacterMovementComponent.MovementMode` (`Character.CharacterMovement` _asbp_adventurer)) "MOVE_None")
    (`self.K2_DestroyActor`)
    (else
      (goto _label))))

(fn `NewFunction`)

(fn `UserConstructionScript`
  (set `ProjectileMovementComponent.InitialSpeed` (`self.Projectile Speed`) (`self.ProjectileMovement`)))