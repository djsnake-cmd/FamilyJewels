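; Player character for the adventurer, moving along world X with double jump, mouse aiming and a grappling hook.
; While Aim is held, Tick projects the mouse ray toward the character's Y plane and rotates the Projectile component toward that point.
; Fire spawns BP_GrappleHook there; MoveGrapple disables movement and lerps the actor between grapple points on a distance-scaled timeline.
; CancelFire or timeline completion restores walking.
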(event `InputAxis|Forward`
  (params (AxisValue :type "Float (single-precision)"))
  (`self.AddMovementInput` (1.0 0.0 0.0) AxisValue))

(event `InputAction|Jump`
  (params (Key :type "Key Structure"))
  (:`Pressed`
    (set `self.JumpMaxCount` 2)
    (`self.Jump`))
  (:`Released`
    (`self.StopJumping`)))

(event `self.OnJumped`
  (`PaperZDAnimInstance.JumpToNode` (`PaperZDAnimationComponent.AnimInstance` (`self.AnimationComponent`)) "Airborne" "None" :!label _label))

(event `self.OnWalkingOffLedge`
  (params (PreviousFloorImpactNormal :type "Vector Structure (by ref)") (PreviousFloorContactNormal :type "Vector Structure (by ref)") (PreviousLocation :type "Vector Structure (by ref)") (TimeDelta :type "Float (single-precision)"))
  (goto _label))

(event `self.ReceiveAnyDamage`
  (params (Damage :type "Float (single-precision)") (DamageType :type "DamageType Object Reference") (InstigatedBy :type "Controller Object Reference") (DamageCauser :type "Actor Object Reference"))
  (`KismetSystemLibrary.PrintString` (`KismetStringLibrary.Conv_DoubleToString` Damage)))

(event `MoveGrapple`
  ;[1 1 1] Set max time for grapple
  (`TimelineComponent.SetPlayRate` (`self.MoveGrappleTL`) (/ 1.0 (`KismetMathLibrary.FClamp` (/ (`KismetMathLibrary.VSize` (+ (`self.GrappleEndLoc`) (`self.GrappleStartLoc`))) 2400.0) 0.1)))
  ;[1 1 1] MoveForward
  (`CharacterMovementComponent.DisableMovement` (`self.CharacterMovement`))
  (bind (_direction _grappletrack) (`Timeline|MoveGrappleTL` :!via `PlayFromStart`)
    (:`Update`
      (`self.K2_SetActorLocation` (`KismetMathLibrary.VLerp` (`self.GrappleStartLoc`) (`self.GrappleEndLoc`) _grappletrack)))
    (:`Finished`
      (`CharacterMovementComponent.SetMovementMode` (`self.CharacterMovement`) "MOVE_Walking" 0)
      (set `self.IsGrappling?` false))))

(event `InputAction|Fire`
  (params (Key :type "Key Structure"))
  (bind (_returnvalue_roll _returnvalue_pitch _returnvalue_yaw) (`KismetMathLibrary.BreakRotator` (`SceneComponent.K2_GetComponentRotation` (`self.CapsuleComponent`))))
  (:`Pressed`
    (if (not (`self.IsGrappling?`))
      (set `self.IsGrappling?` false)
      (bind _returnvalue (`|SpawnActorFromClass` "/Game/Blueprints/Adventurer/BP_GrappleHook.BP_GrappleHook_C" (`SceneComponent.K2_GetComponentToWorld` (`self.Projectile`)) "AdjustIfPossibleButAlwaysSpawn" "OverrideRootScale" null null))
      ;[1 1 1] GrappleFacingFrwd
      (`self.K2_SetActorRotation` _returnvalue (`KismetMathLibrary.MakeRotator` 0.0 0.0 _returnvalue_yaw) false))))

(event `self.ReceiveTick`
  (params (DeltaSeconds :type "Float (single-precision)"))
  (`|ExecutionSequence`
    (:`then_0`
      (`self.GetMousePosition`))))

(event `InputAction|CancelFire`
  (params (Key :type "Key Structure"))
  ;[1 1 1] Cancel Grapple
  (:`Pressed`
    (if (`|EnumEquality` (`CharacterMovementComponent.MovementMode` (`self.CharacterMovement`)) "MOVE_None")
      (`TimelineComponent.Stop` (`self.MoveGrappleTL`))
      (`CharacterMovementComponent.SetMovementMode` (`self.CharacterMovement`) "MOVE_Walking" 0)
      (set `self.IsGrappling?` false))))

(event `InputAction|Aim`
  (params (Key :type "Key Structure"))
  (:`Pressed`
    (set `self.PressAim` true))
  (:`Released`
    (set `self.PressAim` false)))

(event `GetMousePosition`
  (bind _aimyaw (`self.AimYaw`))
  (bind (_worldlocation _worlddirection) (`PlayerController.DeprojectMousePositionToWorld` (`GameplayStatics.GetPlayerController` 0)))
  (bind _returnvalue (+ _worlddirection (* _worlddirection 99999.0)))
  (if (`self.PressAim`)
    (`KismetSystemLibrary.LineTraceMulti` _worldlocation _returnvalue "TraceTypeQuery1")
    (bind _aimpoint (`self.Aim Location` _worldlocation _returnvalue))
    (`KismetSystemLibrary.DrawDebugSphere` _aimpoint 20.0 24 (struct :`R` 0.129583 :`G` 1.0 :`A` 1.0) 0.1)
    (bind (_yaw _pitch) (`KismetMathLibrary.GetYawPitchFromVector` (`KismetMathLibrary.Normal` (- _aimpoint (`SceneComponent.K2_GetComponentLocation` (`self.Projectile`))))))
    (bind _output_get (set `self.AimYaw` _yaw))
    (bind _output_get_2 (set `self.AimPitch` _pitch))
    (`SceneComponent.K2_SetWorldRotation` (`self.Projectile`) (`KismetMathLibrary.MakeRotator` 0.0 _output_get_2 _output_get) false false)
    (if (== (/ _aimyaw (`KismetMathLibrary.Abs` _aimyaw)) 1.0)
      (`self.K2_SetActorRotation` (struct))
      (`SceneComponent.SetWorldScale3D` (`self.Projectile`) (1.0 1.0 1.0))
      (else
        (`self.K2_SetActorRotation` (struct))
        (`SceneComponent.SetWorldScale3D` (`self.Projectile`) (1.0 1.0 1.0))))))

(fn `Aim Location`
  (params (InputLocation :type "Vector Structure" :default (0.0 0.0 0.0)) (`Input Pin` :type "Vector Structure" :default (0.0 0.0 5.0)))
  (returns (AimPoint :type "Vector Structure"))
  (bind _y (.y `Input Pin`))
  (bind _y_2 (.y InputLocation))
  (bind (_returnvalue_x _returnvalue_y) (`KismetMathLibrary.BreakVector` (`self.K2_GetActorLocation`)))
  (return (`KismetMathLibrary.MakeVector` (+ (/ (* (- _returnvalue_y _y_2) (- (.x `Input Pin`) (.x InputLocation))) (- _y _y_2)) 0.0) _returnvalue_y (+ 0.0 (/ (* (- _returnvalue_y _y_2) (- (.z `Input Pin`) (.z InputLocation))) (- _y _y_2))))))

(fn `UserConstructionScript`)